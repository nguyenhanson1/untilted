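; BP_UntitledPlayerController is a player controller that handles team selection before spawning.
; On BeginPlay the server possesses the first BP_StartingView in the level, while the local client shows the W_TeamMenu widget with the mouse cursor visible.
; TeamSelected asks BP_TestGameMode to spawn the player for the chosen team, then switches input to game-only and hides the cursor.
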(event `self.ReceiveBeginPlay`
  (`|ExecutionSequence`
    (:`then_0`
      (`/Engine/EditorBlueprintResources/ActorMacros.Switch Has Authority`
        (:`Authority`
          (bind _outactors (`GameplayStatics.GetAllActorsOfClass` "/Game/Blueprints/PlayerCharacter/BP_StartingView.BP_StartingView_C"))
          (`self.Possess` (`|GetArrayItem` _outactors)))))
    (:`then_1`
      (if (`self.IsLocalPlayerController`)
        (bind _returnvalue (`|CreateWidget` "/Game/Widget/W_TeamMenu.W_TeamMenu_C"))
        (`UserWidget.AddToViewport` _returnvalue 0)
        (set `self.bShowMouseCursor` true)))))

(event `TeamSelected`
  (params (Team :type "ETeamState Enum" :default "TS_None"))
  (bind _asbp_test_game_mode (cast `/Game/Blueprints/GameMode/BP_TestGameMode` (`GameplayStatics.GetGameMode`)))
  (`/Game/Blueprints/GameMode/BP_TestGameMode.RequestSpawn` _asbp_test_game_mode Team self)
  (`WidgetBlueprintLibrary.SetInputMode_GameOnly` self)
  (set `self.bShowMouseCursor` false))

(fn `UserConstructionScript`)