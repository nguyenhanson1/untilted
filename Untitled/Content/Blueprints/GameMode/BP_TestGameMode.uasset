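; BP_TestGameMode is a game mode that spawns and possesses team characters for controllers in a two-team game.
; Its RequestSpawn event branches on the team and scans all BP_UntitledPlayerStart actors for the first one whose TeamB flag matches.
; It spawns that team's character class there with the team assigned, adjusting for collisions but always spawning, and the given controller possesses it.
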(event `RequestSpawn`
  (params (Team :type "ETeamState Enum" :default "TS_None") (Controller :type "PlayerController Object Reference"))
  (switch `ETeamState` Team
    (:`TS_TeamA`
      (bind _outactors (`GameplayStatics.GetAllActorsOfClass` "/Game/Blueprints/PlayerStart/BP_UntitledPlayerStart.BP_UntitledPlayerStart_C"))
      (for _array_element _outactors
        (if (not (`UntitledPlayerStart.bTeamB` _array_element))
          (bind _returnvalue (`|SpawnActorFromClass` "/Game/Blueprints/PlayerCharacter/BP_TeamACharacter.BP_TeamACharacter_C" (`self.GetTransform` _array_element) "AdjustIfPossibleButAlwaysSpawn" "OverrideRootScale" null Team null))
          (`Controller.Possess` Controller _returnvalue)
          (break))))
    (:`TS_TeamB`
      (bind _outactors_2 (`GameplayStatics.GetAllActorsOfClass` "/Game/Blueprints/PlayerStart/BP_UntitledPlayerStart.BP_UntitledPlayerStart_C"))
      (for _array_element_2 _outactors_2
        (if (`UntitledPlayerStart.bTeamB` _array_element_2)
          (bind _returnvalue_2 (`|SpawnActorFromClass` "/Game/Blueprints/PlayerCharacter/BP_TeamBCharacter.BP_TeamBCharacter_C" (`self.GetTransform` _array_element_2) "AdjustIfPossibleButAlwaysSpawn" "OverrideRootScale" null Team null))
          (`Controller.Possess` Controller _returnvalue_2)
          (break))))))

(fn `UserConstructionScript`)