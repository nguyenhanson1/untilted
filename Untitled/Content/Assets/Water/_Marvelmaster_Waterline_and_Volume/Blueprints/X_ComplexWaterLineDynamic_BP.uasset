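; Dynamic waterline actor that renders an underwater cube through a scene capture for the camera.
; The cube's dynamic material receives the water body's heightfield, re-set on timeline updates as a packaged-build workaround.
; Within range, the capture attaches to the camera; beyond it, it detaches, deactivates and clears the render target, allowing multiple instances per world.
; Cube overlaps shorten and restore the overlapping actor's spring arm.
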(event `self.ReceiveBeginPlay`
  (bind _underwatercube (`self.UnderWaterCube`))
  (`SceneCaptureComponent.ShowOnlyComponent` (`self.WaveCapture`) (`self.UnderWaterCube`))
  (`self.SetOwner` (`GameplayStatics.GetPlayerCharacter` 0))
  (`PrimitiveComponent.SetOwnerNoSee` (`self.UnderWaterCube`) true)
  (bind _returnvalue (`PrimitiveComponent.CreateDynamicMaterialInstance` _underwatercube 0 "/Game/Assets/Water/_Marvelmaster_Waterline_and_Volume/Materials/X_ComplexDynamicWaterline/X_WaterLineCubeDynamic_mat.X_WaterLineCubeDynamic_mat" "None"))
  (bind _output_get (set `self.dynmat` _returnvalue))
  (`PrimitiveComponent.SetMaterial` _underwatercube 0 _output_get)
  (bind _outactors (`GameplayStatics.GetAllActorsOfClass` "/Game/Assets/Water/_Marvelmaster_infinite_reactive_water_/Blueprints/WaterBody_BP0.WaterBody_BP0_C"))
  ;[1 1 1] for some reason needs to update all the time in packed project
  (`Timeline|Timeline_0` :!via `PlayFromStart`
    (:`Update`
      (`MaterialInstanceDynamic.SetTextureParameterValue` (`self.dynmat`) "Heightfield" (`/Game/Assets/Water/_Marvelmaster_infinite_reactive_water_/Blueprints/WaterBody_BP0.height` (`|GetArrayItem` _outactors))))))

(event `self.ReceiveTick`
  (params (DeltaSeconds :type "Float (single-precision)"))
  (bind _wavecapture (`self.WaveCapture`))
  (bind _wavecapture_2 (`self.WaveCapture`))
  (bind _playercameramanager (`PlayerController.PlayerCameraManager` (`GameplayStatics.GetPlayerController` 0)))
  (`KismetSystemLibrary.Delay` 0.2)
  (if (<= (`self.GetDistanceTo` _playercameramanager) 1100.0)
    (`/Engine/EditorBlueprintResources/StandardMacros.DoOnce` false :!label _label
      (:`Completed`
        (`SceneComponent.K2_AttachToComponent` _wavecapture_2 (`PlayerCameraManager.TransformComponent` _playercameramanager) "None" "SnapToTarget" "SnapToTarget" "SnapToTarget" true)
        ;[1 1 1] needed to use multiple of these blueprints in world
        (`ActorComponent.Activate` _wavecapture false)
        (goto _label_2 :!via `Reset`)))
    (else
      (`/Engine/EditorBlueprintResources/StandardMacros.DoOnce` false :!label _label_2
        (:`Completed`
          (`SceneComponent.K2_DetachFromComponent` _wavecapture_2 "KeepRelative" "KeepRelative" "KeepRelative" true)
          (`ActorComponent.Deactivate` _wavecapture)
          (`KismetSystemLibrary.Delay` 1.0)
          (`KismetRenderingLibrary.ClearRenderTarget2D` "/Game/Assets/Water/_Marvelmaster_Waterline_and_Volume/Materials/3_ComplexWaterline/3_ComplexWaterLine_RT.3_ComplexWaterLine_RT")
          (goto _label :!via `Reset`))))))

(event `self.UnderWaterCube.OnComponentBeginOverlap`
  (params (OverlappedComponent :type "PrimitiveComponent Object Reference") (OtherActor :type "Actor Object Reference") (OtherComp :type "PrimitiveComponent Object Reference") (OtherBodyIndex :type Integer) (bFromSweep :type Boolean) (SweepResult :type "HitResult Structure (by ref)"))
  (set `SpringArmComponent.TargetArmLength` 300.0 (`self.GetComponentByClass` OtherActor "/Script/Engine.SpringArmComponent")))

(event `self.UnderWaterCube.OnComponentEndOverlap`
  (params (OverlappedComponent :type "PrimitiveComponent Object Reference") (OtherActor :type "Actor Object Reference") (OtherComp :type "PrimitiveComponent Object Reference") (OtherBodyIndex :type Integer))
  (set `SpringArmComponent.TargetArmLength` 500.0 (`self.GetComponentByClass` OtherActor "/Script/Engine.SpringArmComponent")))

(fn `UserConstructionScript`
  ;[1 1 1] Flicker Debug
  (`PrimitiveComponent.SetBoundsScale` (`self.UnderWaterCube`) 20.0))