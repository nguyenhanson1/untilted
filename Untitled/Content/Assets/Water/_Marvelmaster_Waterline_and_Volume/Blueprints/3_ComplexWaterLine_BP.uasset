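; Waterline volume actor that captures a player-hidden cube into a render target to produce a wave-aware waterline.
; WaveCapture sees only that cube, snaps to the player camera when nearby, and detaches and clears the target when far, allowing multiple instances.
; Box overlap toggles the capture's hidden state.
; Optional infinite mode moves the scaled actor with the camera and writes mask location and size to WaterMask_MPC.
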(event `self.ReceiveBeginPlay`
  ;[1 1 1] Show only Waterlinecube to WaveCapture, Hide WaterlineCube from Player
  (`SceneCaptureComponent.ShowOnlyComponent` (`self.WaveCapture`) (`self.WaterlineCube`))
  (`self.SetOwner` (`GameplayStatics.GetPlayerCharacter` 0))
  (`PrimitiveComponent.SetOwnerNoSee` (`self.WaterlineCube`) true)
  (set `self.InitialLocation` (`self.K2_GetActorLocation`))
  ;[1 1 1] set visible ingame cause its set invisible for editor
  (`SceneComponent.SetVisibility` (`self.WaterlineCube`) true false))

(event `self.ReceiveTick`
  (params (DeltaSeconds :type "Float (single-precision)"))
  (bind _wavecapture (`self.WaveCapture`))
  (bind _wavecapture_2 (`self.WaveCapture`))
  (bind _returnvalue (`KismetMathLibrary.Conv_DoubleToLinearColor` (* 1.0 100000.0)))
  (bind _playercameramanager (`PlayerController.PlayerCameraManager` (`GameplayStatics.GetPlayerController` 0)))
  (bind (_returnvalue_x _returnvalue_y) (`KismetMathLibrary.BreakVector` (`PlayerCameraManager.GetCameraLocation` (`PlayerController.PlayerCameraManager` (`GameplayStatics.GetPlayerController` 0)))))
  (`|ExecutionSequence`
    (:`then_0`
      ;[1 1 1] When Camera is near, attach WaveCapture to it
      (`KismetSystemLibrary.Delay` 0.2)
      (if (<= (`self.GetDistanceTo` _playercameramanager) 1100.0)
        (`/Engine/EditorBlueprintResources/StandardMacros.DoOnce` false :!label _label
          (:`Completed`
            (`SceneComponent.K2_AttachToComponent` _wavecapture (`PlayerCameraManager.TransformComponent` _playercameramanager) "None" "SnapToTarget" "SnapToTarget" "SnapToTarget" true)
            ;[1 1 1] needed to use multiple of these blueprints in world
            (`ActorComponent.Activate` _wavecapture_2 false)
            (goto _label_2 :!via `Reset`)))
        (else
          (`/Engine/EditorBlueprintResources/StandardMacros.DoOnce` false :!label _label_2
            (:`Completed`
              (`SceneComponent.K2_DetachFromComponent` _wavecapture "KeepRelative" "KeepRelative" "KeepRelative" true)
              (`ActorComponent.Deactivate` _wavecapture_2)
              (`KismetSystemLibrary.Delay` 1.0)
              (`KismetRenderingLibrary.ClearRenderTarget2D` "/Game/Assets/Water/_Marvelmaster_Waterline_and_Volume/Materials/3_ComplexWaterline/3_ComplexWaterLine_RT.3_ComplexWaterLine_RT")
              (goto _label :!via `Reset`))))))
    (:`then_1`
      ;[0.08707 0.7478 1] Just needed for infinite waterline
      (if (`self.MakeInfinite`)
        (`self.K2_SetActorTransform` (`KismetMathLibrary.MakeTransform` (`KismetMathLibrary.MakeVector` _returnvalue_x _returnvalue_y 1000.0) (struct) (10.0 10.0 10.0)))
        (`KismetMaterialLibrary.SetVectorParameterValue` "/Game/Assets/Water/_Marvelmaster_Waterline_and_Volume/MaterialFunction+Collections/WaterMask_MPC.WaterMask_MPC" "CameraLoc" (`KismetMathLibrary.Conv_VectorToLinearColor` (`KismetMathLibrary.MakeVector` _returnvalue_x _returnvalue_y)))
        (`KismetMaterialLibrary.SetVectorParameterValue` "/Game/Assets/Water/_Marvelmaster_Waterline_and_Volume/MaterialFunction+Collections/WaterMask_MPC.WaterMask_MPC" "MaskSize" (`KismetMathLibrary.Conv_VectorToLinearColor` (`.BoxExtent` (`KismetSystemLibrary.GetComponentBounds` (`self.WaterlinePlane`)))))
        (goto _label_3 :!via `Reset`)
        (else
          (`/Engine/EditorBlueprintResources/StandardMacros.DoOnce` false :!label _label_3
            (:`Completed`
              (`KismetMaterialLibrary.SetVectorParameterValue` "/Game/Assets/Water/_Marvelmaster_Waterline_and_Volume/MaterialFunction+Collections/WaterMask_MPC.WaterMask_MPC" "CameraLoc" _returnvalue)
              (`KismetMaterialLibrary.SetVectorParameterValue` "/Game/Assets/Water/_Marvelmaster_Waterline_and_Volume/MaterialFunction+Collections/WaterMask_MPC.WaterMask_MPC" "MaskSize" _returnvalue))))))))

(event `self.Box.OnComponentBeginOverlap`
  (params (OverlappedComponent :type "PrimitiveComponent Object Reference") (OtherActor :type "Actor Object Reference") (OtherComp :type "PrimitiveComponent Object Reference") (OtherBodyIndex :type Integer) (bFromSweep :type Boolean) (SweepResult :type "HitResult Structure (by ref)"))
  ;[1 1 1] deactivate capture when not in water, capture is initially hidden in BP
  (`SceneComponent.SetHiddenInGame` (`self.WaveCapture`) false false))

(event `self.Box.OnComponentEndOverlap`
  (params (OverlappedComponent :type "PrimitiveComponent Object Reference") (OtherActor :type "Actor Object Reference") (OtherComp :type "PrimitiveComponent Object Reference") (OtherBodyIndex :type Integer))
  ;[1 1 1] deactivate capture when not in water, capture is initially hidden in BP
  (`SceneComponent.SetHiddenInGame` (`self.WaveCapture`) true false))

(fn `UserConstructionScript`
  (bind _returnvalue (`KismetMathLibrary.Conv_DoubleToLinearColor` (* 1.0 100000.0)))
  ;[1 1 1] Flicker Debug
  (`PrimitiveComponent.SetBoundsScale` (`self.WaterlineCube`) 20.0)
  (`KismetMaterialLibrary.SetVectorParameterValue` "/Game/Assets/Water/_Marvelmaster_Waterline_and_Volume/MaterialFunction+Collections/WaterMask_MPC.WaterMask_MPC" "CameraLoc" _returnvalue)
  (`KismetMaterialLibrary.SetVectorParameterValue` "/Game/Assets/Water/_Marvelmaster_Waterline_and_Volume/MaterialFunction+Collections/WaterMask_MPC.WaterMask_MPC" "MaskSize" _returnvalue))