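; Ocean waterline Blueprint that uses a WaveCapture component rendering only its WaterlineCube, which is hidden from the owning player.
; BeginPlay makes the player pawn the owner, then snaps the capture to the camera manager and activates it.
; DoOnce gates are meant to detach the capture and clear its render target beyond a camera distance, supporting multiple instances, but that distance check is unconnected.
; Construction enlarges the cube's bounds against flicker.
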(event `self.ReceiveBeginPlay`
  (bind _wavecapture (`self.WaveCapture`))
  (bind _wavecapture_2 (`self.WaveCapture`))
  (`SceneCaptureComponent.ShowOnlyComponent` _wavecapture (`self.WaterlineCube`))
  (`self.SetOwner` (`GameplayStatics.GetPlayerPawn` 0))
  (`PrimitiveComponent.SetOwnerNoSee` (`self.WaterlineCube`) true)
  (`SceneComponent.SetVisibility` (`self.WaterlineCube`) true false)
  (`SceneComponent.K2_AttachToComponent` _wavecapture (`PlayerCameraManager.TransformComponent` (`PlayerController.PlayerCameraManager` (`GameplayStatics.GetPlayerController` 0))) "None" "SnapToTarget" "SnapToTarget" "SnapToTarget" true :!label _label)
  ;[1 1 1] needed to use multiple of these blueprints in world
  (`ActorComponent.Activate` _wavecapture_2 false)
  (`/Engine/EditorBlueprintResources/StandardMacros.DoOnce` false :!via `Reset`
    (:`Completed`
      (`SceneComponent.K2_DetachFromComponent` _wavecapture "KeepRelative" "KeepRelative" "KeepRelative" true)
      (`ActorComponent.Deactivate` _wavecapture_2)
      (`KismetSystemLibrary.Delay` 1.0)
      (`KismetRenderingLibrary.ClearRenderTarget2D` "/Game/_Marvelmaster_Waterline_and_Volume/Materials/3_ComplexWaterline/3_ComplexWaterLine_RT.3_ComplexWaterLine_RT")
      (`/Engine/EditorBlueprintResources/StandardMacros.DoOnce` false :!via `Reset`
        (:`Completed`
          (goto _label))))))

(event `self.ReceiveTick`
  (params (DeltaSeconds :type "Float (single-precision)")))

(fn `UserConstructionScript`
  ;[1 1 1] Flicker Debug
  (`PrimitiveComponent.SetBoundsScale` (`self.WaterlineCube`) 20.0))